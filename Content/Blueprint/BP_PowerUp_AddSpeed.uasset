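; Arkanoid speed power-up that falls down the screen and speeds up every ball when the player paddle catches it.
; Tick moves it downward at a constant rate, and BeginPlay registers it in the ArkanoidPlayerController's PowerUps list.
; The Box overlap destroys it on paddle or KillZone contact and removes it from that list, boosting the controller's Balls only for the paddle.
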(event `self.ReceiveTick`
  (params (DeltaSeconds :type "Float (single-precision)"))
  ;[1 1 1] Add movement to the PowerUP Object
  (`self.K2_AddActorLocalOffset` (* (* (0.0 0.0 -1.0) 100.0) DeltaSeconds)))

(event `self.Box.OnComponentBeginOverlap`
  (params (OverlappedComponent :type "PrimitiveComponent Object Reference") (OtherActor :type "Actor Object Reference") (OtherComp :type "PrimitiveComponent Object Reference") (OtherBodyIndex :type Integer) (bFromSweep :type Boolean) (SweepResult :type "HitResult Structure (by ref)"))
  (bind _as_arkanoid_player_controller (`self.As Arkanoid Player Controller`))
  ;[1 1 1] Detector
  (`|ExecutionSequence`
    (:`then_0`
      (cast `PlayerPaddle` OtherActor)
      (`self.K2_DestroyActor`)
      (`self.Remove the Power Up from Player Controller`)
      (`/Engine/EditorBlueprintResources/StandardMacros.IsValid` _as_arkanoid_player_controller
        (:`Is Valid`
          (for _array_element (`ArkanoidPlayerController.Balls` _as_arkanoid_player_controller)
            (`Ball.AddSpeed` _array_element 200.0)))))
    (:`then_1`
      (cast `KillZone` OtherActor)
      (`self.K2_DestroyActor`)
      (`self.Remove the Power Up from Player Controller`))))

(event `self.ReceiveBeginPlay`
  (bind _asarkanoid_player_controller (cast `ArkanoidPlayerController` (`GameplayStatics.GetPlayerController` 0)))
  (bind _output_get (set `self.As Arkanoid Player Controller` _asarkanoid_player_controller))
  (`KismetArrayLibrary.Array_Add` (`ArkanoidPlayerController.powerUps` _output_get) self))

(fn `Remove the Power Up from Player Controller`
  (bind _as_arkanoid_player_controller (`self.As Arkanoid Player Controller`))
  (`/Engine/EditorBlueprintResources/StandardMacros.IsValid` _as_arkanoid_player_controller
    (:`Is Valid`
      (`KismetArrayLibrary.Array_RemoveItem` (`ArkanoidPlayerController.powerUps` _as_arkanoid_player_controller) self))))

(fn `UserConstructionScript`)